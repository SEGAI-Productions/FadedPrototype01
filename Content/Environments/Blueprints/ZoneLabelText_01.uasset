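; Zone label actor that shows a text label in the world, kept turned toward the player's camera.
; The construction script applies the LabelName and TextColor variables to the TextRender component.
; Every tick, it sets the text's world rotation to a look-at from the actor's location to the first player camera manager, acting as a billboard.
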(event `self.ReceiveTick`
  (params (DeltaSeconds :type "Float (single-precision)"))
  (`SceneComponent.K2_SetWorldRotation` (`self.TextRender`) (`KismetMathLibrary.FindLookAtRotation` (`self.K2_GetActorLocation`) (`self.K2_GetActorLocation` (`GameplayStatics.GetPlayerCameraManager` 0))) false false))

(fn `UserConstructionScript`
  (bind _textrender (`self.TextRender`))
  (`TextRenderComponent.K2_SetText` _textrender (`self.LabelName`))
  (`TextRenderComponent.SetTextRenderColor` _textrender (`self.TextColor`)))